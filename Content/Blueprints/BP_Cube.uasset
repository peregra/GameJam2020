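; BP_Cube is a sliceable physics cube for a magnet bridge-building puzzle, converting its static mesh to a procedural mesh on BeginPlay.
; Non-magnet cubes hit by two different magnets within a time threshold get sliced and pushed apart, with a tag-based cooldown.
; Opposite-polarity magnets colliding over a BP_Bridge are trimmed at its side planes, and overlapping pieces lock as static.
; Locking also decrements both magnet counts in BP_GameMode.
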(event Custom|ClearOtherHalfTag
  (if (not (Components|ComponentHasTag (stale Collision|EventHit _outotherhalfprocmesh_5) "Locked"))
    (if (Components|ComponentHasTag (stale Collision|EventHit _outotherhalfprocmesh_5) "Positive")
      (Variables|/Script/Engine.ActorComponent|SetComponentTags (stale Collision|EventHit _outotherhalfprocmesh_5) (Variables|Default|GetPositiveTags))
      (elif (Components|ComponentHasTag (stale Collision|EventHit _outotherhalfprocmesh_5) "Negative")
        (Variables|/Script/Engine.ActorComponent|SetComponentTags (stale Collision|EventHit _outotherhalfprocmesh_5) (Variables|Default|GetNegativeTags))
        (else
          (Variables|/Script/Engine.ActorComponent|SetComponentTags (stale Collision|EventHit _outotherhalfprocmesh_5) (Variables|Default|GetEmpty)))))))

(event Custom|ClearTag
  (if (not (Components|ComponentHasTag (stale Collision|EventHit _asprocedural_mesh_component) "Locked"))
    (if (Components|ComponentHasTag (stale Collision|EventHit _asprocedural_mesh_component) "Positive")
      (Variables|/Script/Engine.ActorComponent|SetComponentTags (stale Collision|EventHit _asprocedural_mesh_component) (Variables|Default|GetPositiveTags))
      (elif (Components|ComponentHasTag (stale Collision|EventHit _asprocedural_mesh_component) "Negative")
        (Variables|/Script/Engine.ActorComponent|SetComponentTags (stale Collision|EventHit _asprocedural_mesh_component) (Variables|Default|GetNegativeTags))
        (else
          (Variables|/Script/Engine.ActorComponent|SetComponentTags (stale Collision|EventHit _asprocedural_mesh_component) (Variables|Default|GetEmpty)))))))

(event EventBeginPlay
  (Utilities|IsValid (Components|GetOwner)
    (:Is%20Not%20Valid
      (Class|KismetProceduralMeshLibrary|CopyProceduralMeshfromStaticMeshComponent (Variables|Default|GetCube) 0 (Variables|Default|GetProceduralMesh) true)
      (Components|DestroyComponent (Variables|Default|GetCube)))))

(event Collision|EventActorBeginOverlap
  (params (OtherActor :type Actor%20Object%20Reference)))

(event EventTick
  (params (DeltaSeconds :type Float%20%28single-precision%29)))

(event Collision|EventHit
  (params (MyComp :type Primitive%20Component%20Object%20Reference) (Other :type Actor%20Object%20Reference) (OtherComp :type Primitive%20Component%20Object%20Reference) (bSelfMoved :type Boolean) (HitLocation :type Vector :default "0, 0, 0") (HitNormal :type Vector :default "0, 0, 0") (NormalImpulse :type Vector :default "0, 0, 0") (Hit :type Hit%20Result%20Structure%20%28by%20ref%29))
  (bind _breakcooldown (Variables|Default|GetBreakCooldown))
  ;[1 1 1] Check if touching two other magnitized cubes, then break
  (bind _asprocedural_mesh_component (Utilities|Casting|CastToProceduralMeshComponent MyComp))
  (if (Components|ComponentHasTag _asprocedural_mesh_component "Magnet")
    ;[1 1 1] Check for opposite polarity collisions, then check bridge overlap and lock in place
    (bind _asprocedural_mesh_component_2 (Utilities|Casting|CastToProceduralMeshComponent OtherComp))
    (if (Components|ComponentHasTag _asprocedural_mesh_component_2 "Magnet")
      (if (not (Math|Boolean|Equal(Boolean) (Components|ComponentHasTag _asprocedural_mesh_component "Positive") (Components|ComponentHasTag _asprocedural_mesh_component_2 "Positive")))
        (bind _outactors (Actor|GetAllActorsOfClass "/Game/Blueprints/BP_Bridge.BP_Bridge_C"))
        (for _array_element _outactors
          (if (or (Class|PrimitiveComponent|IsOverlappingComponent (Variables|/Game/Blueprints/BP_Bridge.BP_Bridge_C|GetOverBridge _array_element) _asprocedural_mesh_component) (Class|PrimitiveComponent|IsOverlappingComponent (Variables|/Game/Blueprints/BP_Bridge.BP_Bridge_C|GetOverBridge _array_element) _asprocedural_mesh_component_2))
            (Utilities|FlowControl|Sequence
              (:then_0
                (if (Class|PrimitiveComponent|IsOverlappingComponent (Variables|/Game/Blueprints/BP_Bridge.BP_Bridge_C|GetSide1 _array_element) _asprocedural_mesh_component)
                  (bind _outotherhalfprocmesh (Class|KismetProceduralMeshLibrary|SliceProceduralMesh _asprocedural_mesh_component (Transformation|GetWorldLocation (Variables|/Game/Blueprints/BP_Bridge.BP_Bridge_C|GetSide1 _array_element)) (Math|Vector|GetRightVector (Variables|/Game/Blueprints/BP_Bridge.BP_Bridge_C|GetSide1 _array_element)) true "UseLastSectionForCap" "/Game/Blueprints/M_Cut.M_Cut"))
                  (CallFunction|SetDefaultPhysics _outotherhalfprocmesh)
                  (Physics|AddImpulse _outotherhalfprocmesh (* (Math|Vector|GetRightVector (Variables|/Game/Blueprints/BP_Bridge.BP_Bridge_C|GetSide1 _array_element)) (Variables|Default|GetBreakImpulse)) "None" false)
                  (bind _asbp_cube (Utilities|Casting|CastToBP_Cube (Components|GetOwner _outotherhalfprocmesh)))
                  (CallFunction|SetNormalMaterial _asbp_cube _outotherhalfprocmesh)))
              (:then_1
                (if (Class|PrimitiveComponent|IsOverlappingComponent (Variables|/Game/Blueprints/BP_Bridge.BP_Bridge_C|GetSide2 _array_element) _asprocedural_mesh_component)
                  (bind _outotherhalfprocmesh_2 (Class|KismetProceduralMeshLibrary|SliceProceduralMesh _asprocedural_mesh_component (Transformation|GetWorldLocation (Variables|/Game/Blueprints/BP_Bridge.BP_Bridge_C|GetSide2 _array_element)) (Math|Vector|GetRightVector (Variables|/Game/Blueprints/BP_Bridge.BP_Bridge_C|GetSide2 _array_element)) true "UseLastSectionForCap" "/Game/Blueprints/M_Cut.M_Cut"))
                  (CallFunction|SetDefaultPhysics _outotherhalfprocmesh_2)
                  (Physics|AddImpulse _outotherhalfprocmesh_2 (* (Math|Vector|GetRightVector (Variables|/Game/Blueprints/BP_Bridge.BP_Bridge_C|GetSide2 _array_element)) (Variables|Default|GetBreakImpulse)) "None" false)
                  (bind _asbp_cube_2 (Utilities|Casting|CastToBP_Cube (Components|GetOwner _outotherhalfprocmesh_2)))
                  (CallFunction|SetNormalMaterial _asbp_cube_2 _outotherhalfprocmesh_2)))
              (:then_2
                (if (Class|PrimitiveComponent|IsOverlappingComponent (Variables|/Game/Blueprints/BP_Bridge.BP_Bridge_C|GetSide1 _array_element) _asprocedural_mesh_component_2)
                  (bind _outotherhalfprocmesh_3 (Class|KismetProceduralMeshLibrary|SliceProceduralMesh _asprocedural_mesh_component_2 (Transformation|GetWorldLocation (Variables|/Game/Blueprints/BP_Bridge.BP_Bridge_C|GetSide1 _array_element)) (Math|Vector|GetRightVector (Variables|/Game/Blueprints/BP_Bridge.BP_Bridge_C|GetSide1 _array_element)) true "UseLastSectionForCap" "/Game/Blueprints/M_Cut.M_Cut"))
                  (CallFunction|SetDefaultPhysics _outotherhalfprocmesh_3)
                  (Physics|AddImpulse _outotherhalfprocmesh_3 (* "0, 0, 0" (Variables|Default|GetBreakImpulse)) "None" false)
                  (bind _asbp_cube_3 (Utilities|Casting|CastToBP_Cube (Components|GetOwner _outotherhalfprocmesh_3)))
                  (CallFunction|SetNormalMaterial _asbp_cube_3 _outotherhalfprocmesh_3)))
              (:then_3
                (if (Class|PrimitiveComponent|IsOverlappingComponent (Variables|/Game/Blueprints/BP_Bridge.BP_Bridge_C|GetSide2 _array_element) _asprocedural_mesh_component_2)
                  (bind _outotherhalfprocmesh_4 (Class|KismetProceduralMeshLibrary|SliceProceduralMesh _asprocedural_mesh_component_2 (Transformation|GetWorldLocation (Variables|/Game/Blueprints/BP_Bridge.BP_Bridge_C|GetSide2 _array_element)) (Math|Vector|GetRightVector (Variables|/Game/Blueprints/BP_Bridge.BP_Bridge_C|GetSide2 _array_element)) true "UseLastSectionForCap" "/Game/Blueprints/M_Cut.M_Cut"))
                  (CallFunction|SetDefaultPhysics _outotherhalfprocmesh_4)
                  (Physics|AddImpulse _outotherhalfprocmesh_4 (* "0, 0, 0" (Variables|Default|GetBreakImpulse)) "None" false)
                  (bind _asbp_cube_4 (Utilities|Casting|CastToBP_Cube (Components|GetOwner _outotherhalfprocmesh_4)))
                  (CallFunction|SetNormalMaterial _asbp_cube_4 _outotherhalfprocmesh_4)))
              (:then_4
                (if (Class|PrimitiveComponent|IsOverlappingComponent (Variables|/Game/Blueprints/BP_Bridge.BP_Bridge_C|GetOverBridge _array_element) _asprocedural_mesh_component)
                  (CallFunction|Lock _asprocedural_mesh_component)
                  (else
                    (CallFunction|SetNormalMaterial _asprocedural_mesh_component)
                    (Variables|/Script/Engine.ActorComponent|SetComponentTags _asprocedural_mesh_component (Variables|Default|GetEmpty)))))
              (:then_5
                (if (Class|PrimitiveComponent|IsOverlappingComponent (Variables|/Game/Blueprints/BP_Bridge.BP_Bridge_C|GetOverBridge _array_element) _asprocedural_mesh_component_2)
                  (CallFunction|Lock _asprocedural_mesh_component_2)
                  (else
                    (CallFunction|SetNormalMaterial _asprocedural_mesh_component_2)
                    (Variables|/Script/Engine.ActorComponent|SetComponentTags _asprocedural_mesh_component_2 (Variables|Default|GetEmpty)))))
              (:then_6
                (CallFunction|FinishLock)))))))
    (elif (not (Components|ComponentHasTag _asprocedural_mesh_component "JustBroke"))
      (bind _asprocedural_mesh_component_3 (Utilities|Casting|CastToProceduralMeshComponent OtherComp))
      (if (Components|ComponentHasTag _asprocedural_mesh_component_3 "Magnet")
        (Utilities|IsValid (Variables|Default|GetLastMagnetHit)
          (:Is%20Valid
            (if (== _asprocedural_mesh_component_3 (Variables|Default|GetLastMagnetHit))
              (Variables|Default|SetTimeMagnetHit (Utilities|Time|GetTimeSeconds))
              (elif (<= (- (Utilities|Time|GetTimeSeconds) (Variables|Default|GetTimeMagnetHit)) (Variables|Default|GetHitTimeThreshold))
                (Utilities|Time|SetTimerbyEvent (delegate Custom|ClearTag) _breakcooldown)
                (Variables|/Script/Engine.ActorComponent|SetComponentTags _asprocedural_mesh_component (Variables|Default|GetBrokeTags))
                (bind _outotherhalfprocmesh_5 (Class|KismetProceduralMeshLibrary|SliceProceduralMesh _asprocedural_mesh_component (+ (Transformation|GetWorldLocation (Variables|Default|GetLastMagnetHit)) (/ (- (Transformation|GetWorldLocation (Variables|Default|GetLastMagnetHit)) (Transformation|GetWorldLocation _asprocedural_mesh_component_3)) 2.0)) (Math|Vector|RotateVectorAroundAxis (- (Transformation|GetWorldLocation (Variables|Default|GetLastMagnetHit)) (Transformation|GetWorldLocation _asprocedural_mesh_component_3)) 9e+01 "0, 0,1.000000") true "CreateNewSectionForCap" "/Game/Blueprints/M_Cut.M_Cut"))
                (Utilities|Time|SetTimerbyEvent (delegate Custom|ClearOtherHalfTag) _breakcooldown)
                (Variables|/Script/Engine.ActorComponent|SetComponentTags _outotherhalfprocmesh_5 (Variables|Default|GetBrokeTags))
                (CallFunction|SetDefaultPhysics _outotherhalfprocmesh_5)
                (Physics|AddImpulse _asprocedural_mesh_component (* (Math|Vector|GetUnitDirection(Vector) (+ (Transformation|GetWorldLocation (Variables|Default|GetLastMagnetHit)) (/ (- (Transformation|GetWorldLocation (Variables|Default|GetLastMagnetHit)) (Transformation|GetWorldLocation _asprocedural_mesh_component_3)) 2.0)) (Transformation|GetWorldLocation _asprocedural_mesh_component)) (Variables|Default|GetBreakImpulse)) "None" false)
                (Physics|AddImpulse _outotherhalfprocmesh_5 (* (Math|Vector|GetUnitDirection(Vector) (+ (Transformation|GetWorldLocation (Variables|Default|GetLastMagnetHit)) (/ (- (Transformation|GetWorldLocation (Variables|Default|GetLastMagnetHit)) (Transformation|GetWorldLocation _asprocedural_mesh_component_3)) 2.0)) (Transformation|GetWorldLocation _outotherhalfprocmesh_5)) (Variables|Default|GetBreakImpulse)) "None" false))))
          (:Is%20Not%20Valid
            (Variables|Default|SetLastMagnetHit _asprocedural_mesh_component_3)
            (Variables|Default|SetTimeMagnetHit (Utilities|Time|GetTimeSeconds))))))))

(fn ConstructionScript)

(fn SetDefaultPhysics
  (params (SetMesh :type Procedural%20Mesh%20Component%20Object%20Reference))
  (Utilities|IsValid SetMesh
    (:Is%20Valid
      (Physics|SetSimulatePhysics SetMesh true)
      (Collision|SetCollisionObjectType SetMesh "ECC_WorldDynamic")
      (Class|PrimitiveComponent|SetConstraintMode SetMesh "XYPlane")
      (Class|PrimitiveComponent|SetNotifyRigidBodyCollision SetMesh true))))

(fn Lock
  (params (LockThis :type Procedural%20Mesh%20Component%20Object%20Reference))
  (Variables|/Script/Engine.ActorComponent|SetComponentTags LockThis (Variables|Default|GetLocked))
  (bind _asbp_cube (Utilities|Casting|CastToBP_Cube (Components|GetOwner LockThis)))
  (CallFunction|SetLockedMaterial _asbp_cube LockThis)
  (Physics|SetSimulatePhysics LockThis false)
  (Collision|SetCollisionObjectType LockThis "ECC_WorldStatic"))

(fn PlayLockSound)

(fn FinishLock
  (bind _asbp_game_mode (Utilities|Casting|CastToBP_GameMode (Game|GetGameMode)))
  (Variables|/Game/Blueprints/BP_GameMode.BP_GameMode_C|SetPositiveMagnets _asbp_game_mode (- (Variables|/Game/Blueprints/BP_GameMode.BP_GameMode_C|GetPositiveMagnets _asbp_game_mode) 1))
  (Variables|/Game/Blueprints/BP_GameMode.BP_GameMode_C|SetNegativeMagnets _asbp_game_mode (- (Variables|/Game/Blueprints/BP_GameMode.BP_GameMode_C|GetNegativeMagnets _asbp_game_mode) 1))
  (CallFunction|PlayLockSound))

(fn SetLockedMaterial
  (params (ProceduralMesh :type Procedural%20Mesh%20Component%20Object%20Reference))
  (Rendering|Material|SetMaterial ProceduralMesh 0 "/Game/Blueprints/M_Locked.M_Locked"))

(fn SetNormalMaterial
  (params (ProceduralMesh :type Procedural%20Mesh%20Component%20Object%20Reference))
  (Rendering|Material|SetMaterial ProceduralMesh 0 "/Game/Blueprints/M_Cube.M_Cube"))

(fn SetNegativeMaterial
  (params (NewParam :type Procedural%20Mesh%20Component%20Object%20Reference))
  (Rendering|Material|SetMaterial NewParam 0 "/Game/Blueprints/M_Negative.M_Negative"))

(fn SetPositiveMaterial
  (params (NewParam :type Procedural%20Mesh%20Component%20Object%20Reference))
  (Rendering|Material|SetMaterial NewParam 0 "/Game/Blueprints/M_Positive.M_Positive"))