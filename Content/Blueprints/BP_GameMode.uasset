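; Game mode that respawns the first-person character and simulates magnetism between magnet-tagged procedural meshes on BP_Cube actors.
; When the character is destroyed, it spawns and possesses a replacement after a short delay, then rebinds the destroy event.
; With multiple magnets, a looping timer rebuilds the magnet list.
; Tick applies pairwise forces, inversely proportional to distance, repelling like and attracting opposite polarities; Locked magnets receive no force.
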(event Custom|UpdateCurrentMagnets
  (if (> (+ (Variables|Default|GetPositiveMagnets) (Variables|Default|GetNegativeMagnets)) 1)
    (Utilities|Array|Clear (Variables|Default|GetMagnetArray))
    (bind _outactors (Actor|GetAllActorsOfClass "/Game/Blueprints/BP_Cube.BP_Cube_C"))
    (for _array_element _outactors
      (for _array_element_2 (Actor|GetComponentsbyTag _array_element "/Script/ProceduralMeshComponent.ProceduralMeshComponent" "Magnet")
        (Utilities|Array|Add (Variables|Default|GetMagnetArray) _array_element_2)))))

(event Custom|Death%20Delay
  (params (DestroyedActor :type Actor%20Object%20Reference))
  (Utilities|FlowControl|Delay 0.5)
  (bind _returnvalue (Game|SpawnActorfromClass "/Game/FirstPersonCPP/Blueprints/FirstPersonCharacter.FirstPersonCharacter_C" (Variables|Default|GetSpawnTransform) "Undefined" 0 0))
  (Pawn|Possess (Game|GetPlayerController 0) _returnvalue)
  (CallFunction|Respawn))

(event Custom|Respawn
  (bind _asfirst_person_character (Utilities|Casting|CastToFirstPersonCharacter (Game|GetPlayerCharacter 0)))
  (Game|BindEventtoOnDestroyed _asfirst_person_character (delegate Custom|Death%20Delay)))

(event EventBeginPlay
  (Utilities|Time|SetTimerbyEvent (delegate Custom|UpdateCurrentMagnets) 0.1 true)
  (bind _asfirst_person_character (Utilities|Casting|CastToFirstPersonCharacter (Game|GetPlayerCharacter 0)))
  (Game|BindEventtoOnDestroyed _asfirst_person_character (delegate Custom|Death%20Delay)))

(event EventTick
  (params (DeltaSeconds :type Float%20%28single-precision%29))
  (if (> (+ (Variables|Default|GetPositiveMagnets) (Variables|Default|GetNegativeMagnets)) 1)
    (CallFunction|ApplyMagnetForces DeltaSeconds)))

(fn ConstructionScript)

(fn ApplyMagnetForces
  (params (DeltaSeconds :type Float%20%28single-precision%29))
  (bind _magnetarray (Variables|Default|GetMagnetArray))
  (for (_array_element _array_index) _magnetarray
    (if (not (Components|ComponentHasTag _array_element "Locked"))
      (for (_array_element_2 _array_index_2) _magnetarray
        (if (not (== _array_index _array_index_2))
          (if (Math|Boolean|Equal(Boolean) (Components|ComponentHasTag _array_element "Positive") (Components|ComponentHasTag _array_element_2 "Positive"))
            ;[1 1 1] Repel
            (Physics|AddForce _array_element (* (Math|Vector|GetUnitDirection(Vector) (Transformation|GetWorldLocation _array_element_2) (Transformation|GetWorldLocation _array_element)) (* DeltaSeconds (/ (Variables|Default|GetMagnetStrength) (/ (Math|Vector|Distance(Vector) (Transformation|GetWorldLocation _array_element_2) (Transformation|GetWorldLocation _array_element)) 1e+03)))) "None" false)
            (else
              ;[1 1 1] Attract
              (Physics|AddForce _array_element (* (Math|Vector|GetUnitDirection(Vector) (Transformation|GetWorldLocation _array_element) (Transformation|GetWorldLocation _array_element_2)) (* DeltaSeconds (/ (Variables|Default|GetMagnetStrength) (/ (Math|Vector|Distance(Vector) (Transformation|GetWorldLocation _array_element) (Transformation|GetWorldLocation _array_element_2)) 1e+03)))) "None" false))))))))