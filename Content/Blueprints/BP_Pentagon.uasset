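; BP_Pentagon is a pentagon shape Blueprint that supplies the materials for its visual states: normal, positive, negative and locked.
; Each state has its own event, which receives a mesh and sets material slots 0 and 1 on it.
; Normal pairs the pentagon material with the cube material, while the other states use one material for both slots.
; The file holds no other active gameplay logic.
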(event EventBeginPlay
  (|CallParentFunction) ; This node is disabled and will not be called.\nDrag off pins to build functionality.
)

(event Collision|EventActorBeginOverlap
  (params (OtherActor :type Actor%20Object%20Reference))
  (|CallParentFunction OtherActor) ; This node is disabled and will not be called.\nDrag off pins to build functionality.
)

(event EventTick
  (params (DeltaSeconds :type Float%20%28single-precision%29))
  (|CallParentFunction DeltaSeconds) ; This node is disabled and will not be called.\nDrag off pins to build functionality.
)

(event EventSetNormalMaterial
  (params (ProceduralMesh :type Procedural%20Mesh%20Component%20Object%20Reference))
  (Rendering|Material|SetMaterial ProceduralMesh 0 "/Game/Blueprints/M_Pentagon.M_Pentagon")
  (Rendering|Material|SetMaterial ProceduralMesh 1 "/Game/Blueprints/M_Cube.M_Cube"))

(event EventSetPositiveMaterial
  (params (NewParam :type Procedural%20Mesh%20Component%20Object%20Reference))
  (Rendering|Material|SetMaterial NewParam 0 "/Game/Blueprints/M_Positive.M_Positive")
  (Rendering|Material|SetMaterial NewParam 1 "/Game/Blueprints/M_Positive.M_Positive"))

(event EventSetNegativeMaterial
  (params (NewParam :type Procedural%20Mesh%20Component%20Object%20Reference))
  (Rendering|Material|SetMaterial NewParam 0 "/Game/Blueprints/M_Negative.M_Negative")
  (Rendering|Material|SetMaterial NewParam 1 "/Game/Blueprints/M_Negative.M_Negative"))

(event EventSetLockedMaterial
  (params (ProceduralMesh :type Procedural%20Mesh%20Component%20Object%20Reference))
  (Rendering|Material|SetMaterial ProceduralMesh 0 "/Game/Blueprints/M_Locked_Pentagon.M_Locked_Pentagon")
  (Rendering|Material|SetMaterial ProceduralMesh 1 "/Game/Blueprints/M_Locked_Pentagon.M_Locked_Pentagon"))

(fn ConstructionScript
  (|CallParentFunction))