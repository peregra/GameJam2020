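; BP_Triangle is a triangle Blueprint that provides material switching for procedural meshes to show locked, negative, normal and positive states.
; Each state has an event that receives a mesh and sets material slots 0 and 1.
; The normal state uses separate triangle and cube materials, while the other states apply one material to both slots.
; It has no active gameplay logic of its own, and its construction script only calls the parent.
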(event EventBeginPlay
  (|CallParentFunction) ; This node is disabled and will not be called.\nDrag off pins to build functionality.
)

(event Collision|EventActorBeginOverlap
  (params (OtherActor :type Actor%20Object%20Reference))
  (|CallParentFunction OtherActor) ; This node is disabled and will not be called.\nDrag off pins to build functionality.
)

(event EventTick
  (params (DeltaSeconds :type Float%20%28single-precision%29))
  (|CallParentFunction DeltaSeconds) ; This node is disabled and will not be called.\nDrag off pins to build functionality.
)

(event EventSetLockedMaterial
  (params (ProceduralMesh :type Procedural%20Mesh%20Component%20Object%20Reference))
  (Rendering|Material|SetMaterial ProceduralMesh 0 "/Game/Blueprints/M_Locked_Triangle.M_Locked_Triangle")
  (Rendering|Material|SetMaterial ProceduralMesh 1 "/Game/Blueprints/M_Locked_Triangle.M_Locked_Triangle"))

(event EventSetNegativeMaterial
  (params (NewParam :type Procedural%20Mesh%20Component%20Object%20Reference))
  (Rendering|Material|SetMaterial NewParam 0 "/Game/Blueprints/M_Negative.M_Negative")
  (Rendering|Material|SetMaterial NewParam 1 "/Game/Blueprints/M_Negative.M_Negative"))

(event EventSetNormalMaterial
  (params (ProceduralMesh :type Procedural%20Mesh%20Component%20Object%20Reference))
  (Rendering|Material|SetMaterial ProceduralMesh 0 "/Game/Blueprints/M_Triangle.M_Triangle")
  (Rendering|Material|SetMaterial ProceduralMesh 1 "/Game/Blueprints/M_Cube.M_Cube"))

(event EventSetPositiveMaterial
  (params (NewParam :type Procedural%20Mesh%20Component%20Object%20Reference))
  (Rendering|Material|SetMaterial NewParam 0 "/Game/Blueprints/M_Positive.M_Positive")
  (Rendering|Material|SetMaterial NewParam 1 "/Game/Blueprints/M_Positive.M_Positive"))

(fn ConstructionScript
  (|CallParentFunction))